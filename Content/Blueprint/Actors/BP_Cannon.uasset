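; BP_Cannon is a cannon actor that fires projectiles automatically and repeatedly from BeginPlay.
; Each shot spawns a scaled projectile at the ProjectileSpawnPoint's location and rotation, then plays CannonFireRateTimeline from the start.
; The timeline slides the barrel along its relative X, and its Cannon Fired event waits for the CannonFireRate delay before looping back to the next shot.
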(event EventBeginPlay
  ;[1 0.3018 0.3217] Spawns a projectile based on the rate of fire
  (CallFunction|SpawnProjectile :!label _label)
  ;[0.09543 1 0.1731] Animate the barrel during firing and then loop back to fire again
  (bind _fireanimationprogress (Timeline|CannonFireRateTimeline PlayFromStart)
    (:Update
      (CallFunction|AnimateCannonBarrel _fireanimationprogress))
    (:CannonFired
      (Utilities|FlowControl|Delay (Variables|CannonProperties|GetCannonFireRate))
      (goto _label))))

(fn ConstructionScript)

(fn SpawnProjectile
  (bind _projectilespawnpoint (Variables|Default|GetProjectileSpawnPoint))
  (Game|SpawnActorfromClass "/Game/Blueprint/Actors/Projectiles/BP_CannonBall.BP_Cannonball_C" (Math|Transform|MakeTransform (Transformation|GetWorldLocation _projectilespawnpoint) (Transformation|GetWorldRotation _projectilespawnpoint) (Math|Conversions|ToVector(Float) (Variables|CannonProperties|GetCannonballScale))) "Undefined" 0 0))

(fn AnimateCannonBarrel
  (params (BarrelLocation :type Float%20%28single-precision%29))
  (Transformation|SetRelativeLocation (Variables|Default|GetCannonBarrel) (Math|Vector|MakeVector BarrelLocation 0.0 0.0) false false))