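; Collectable crystal powerup actor that is pulled into the player on overlap and then destroys itself, with no reward logic in this Blueprint.
; An IsPlayer check gates the overlap, then the crystal caches its location, scale and light intensity and plays CollectionTimeline.
; Separate timeline tracks drive lerps that home it toward the pawn's current location, shrink it and fade its light before destruction.
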(event Collision|EventActorBeginOverlap
  (params (OtherActor :type Actor%20Object%20Reference))
  ;[0 0 1] Collects crystal powerups when the player approaches them and destroys the powerup
  (Utilities|IsPlayer OtherActor
    (:IsPlayer
      (CallFunction|StoreStartingValues)
      (bind (_direction _collectionprogress _scaleprogress _lightintensityprogress) (Timeline|CollectionTimeline Play)
        (:Update
          (CallFunction|MovetoPlayer _collectionprogress (Game|Player|GetPlayerPawn 0))
          (CallFunction|ShrinkScaletoZero _scaleprogress)
          (CallFunction|FadeLighttoZero _lightintensityprogress))
        (:Finished
          (Actor|DestroyActor))))))

(fn ConstructionScript)

(fn MovetoPlayer
  (params (CollectionProgress :type Float%20%28single-precision%29) (PlayerPawn :type Actor%20Object%20Reference))
  (Transformation|SetActorLocation (Math|Vector|Lerp(Vector) (Variables|Default|GetStartLocation) (Transformation|GetActorLocation PlayerPawn) CollectionProgress) false false))

(fn StoreStartingValues
  ;[1 0.9396 0.1073] Stores starting values for Player Pawn location and the 3D scale and light intensity of the Crystal
  (Variables|Default|SetStartLocation (Transformation|GetActorLocation))
  (Variables|Default|SetStartScale (Transformation|GetActorScale3D))
  (Variables|Default|SetStartingIntensity (Variables|/Script/Engine.LightComponentBase|GetIntensity (Variables|Default|GetCrystalLight))))

(fn ShrinkScaletoZero
  (params (ScaleProgress :type Float%20%28single-precision%29))
  (Transformation|SetActorScale3D (Math|Vector|Lerp(Vector) (Variables|Default|GetStartScale) "0, 0, 0" ScaleProgress)))

(fn FadeLighttoZero
  (params (Alpha :type Float%20%28single-precision%29))
  (Rendering|Components|Light|SetIntensity (Variables|Default|GetCrystalLight) (Math|Float|Lerp (Variables|Default|GetStartingIntensity) 0.0 Alpha)))