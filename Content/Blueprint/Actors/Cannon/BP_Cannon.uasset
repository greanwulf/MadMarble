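; Cannon actor that fires BP_CannonBall projectiles automatically and repeatedly from BeginPlay.
; Each cycle waits CannonRoF, then spawns a ball at BallSpawnPoint's location and rotation, sized by ProjectileScale.
; The AnimateBarrel timeline then slides the barrel along its relative X axis, and its Cannon Fired event restarts the cycle.
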(event EventBeginPlay
  (bind _ballspawnpoint (Variables|Default|GetBallSpawnPoint))
  (Utilities|FlowControl|Delay (Variables|CannonProperties|GetCannonRoF) :!label _label)
  (Game|SpawnActorfromClass "/Game/Blueprint/Actors/Cannon/BP_CannonBall.BP_CannonBall_C" (Math|Transform|MakeTransform (Transformation|GetWorldLocation _ballspawnpoint) (Transformation|GetWorldRotation _ballspawnpoint) (Math|Conversions|ToVector(Float) (Variables|CannonProperties|GetProjectileScale))) "Undefined" 0 0)
  (bind _animatebarrel (Timeline|AnimateBarrel PlayFromStart)
    (:Update
      (Transformation|SetRelativeLocation (Variables|Default|GetCannonBarrel) (Math|Vector|MakeVector _animatebarrel 0.0 0.0) false false))
    (:CannonFired
      (goto _label))))

(fn ConstructionScript)