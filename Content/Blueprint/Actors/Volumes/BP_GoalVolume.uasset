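; BP_GoalVolume is a level goal volume, apparently an unfinished level exit for a crystal-collection game.
; On overlap by the player, it checks whether any BP_Crystal actors remain, but nothing follows that check.
; Helper functions find the current level in a LevelNames array, detect the final one and open the next by name.
; CompleteLevel is an empty stub, and LoadNextLevel is never called here.
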(event Collision|EventActorBeginOverlap
  (params (OtherActor :type Actor%20Object%20Reference))
  (Utilities|IsPlayer OtherActor
    (:IsPlayer
      (if (CallFunction|CheckCrystalsRemaining)
        _))))

(fn ConstructionScript)

(fn CheckCrystalsRemaining
  (bind _outactors (Actor|GetAllActorsOfClass "/Game/Blueprint/Actors/Collectables/BP_Crystal.BP_Crystal_C"))
  (return (> (Utilities|Array|Length _outactors) 0)))

(fn IsFinalLevel
  (return (== (Utilities|Array|LastIndex (Variables|Default|GetLevelNames)) (CallFunction|GetCurrentLevelIndex))))

(fn GetCurrentLevelIndex
  (bind _returnvalue (Game|GetCurrentLevelName true))
  (return (Utilities|Array|FindItem (Variables|Default|GetLevelNames) (Utilities|String|StringToName _returnvalue))))

(fn CompleteLevel)

(fn LoadNextLevel
  (Game|OpenLevel(byName) (CallFunction|GetNextLevelName)))

(fn GetNextLevelName
  (bind _result (Math|Integer|IncrementInt (CallFunction|GetCurrentLevelIndex))
    (:%20%20
      (return (Utilities|Array|Get(acopy) (Variables|Default|GetLevelNames) _result)))))